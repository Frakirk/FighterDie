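; Death_Die is a physics die actor that knocks the player away when the player hits it.
; A hit on its Cube from a PlayerCharacter calls Bounce, which pushes the mesh away with upward lift and random spin, then launches the character away from the die and upward.
; SetColour tints the die by applying a dynamic material instance with a CustomColour parameter to the mesh.
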(event OnComponentHit(Cube)
  (params (HitComponent :type Primitive%20Component%20Object%20Reference) (OtherActor :type Actor%20Object%20Reference) (OtherComp :type Primitive%20Component%20Object%20Reference) (NormalImpulse :type Vector :default "0, 0, 0") (Hit :type Hit%20Result%20Structure%20%28by%20ref%29))
  (bind _asplayer_character (Utilities|Casting|CastToPlayerCharacter OtherActor))
  (CallFunction|Bounce _asplayer_character 1.0)
  (Character|LaunchCharacter _asplayer_character (Math|Vector|MakeVector (.X (Math|Vector|BreakVector (* (Math|Vector|GetUnitDirection(Vector) (Transformation|GetWorldLocation (Variables|Default|GetStaticMesh)) (Transformation|GetActorLocation _asplayer_character)) 5e+02))) (.Y (Math|Vector|BreakVector (* (Math|Vector|GetUnitDirection(Vector) (Transformation|GetWorldLocation (Variables|Default|GetStaticMesh)) (Transformation|GetActorLocation _asplayer_character)) 5e+02))) 2.5e+02) true true))

(event Custom|Bounce
  (params (OtherActor :type Actor%20Object%20Reference) (ForceScale :type Float%20%28single-precision%29))
  (bind _returnvalue (Transformation|GetActorLocation OtherActor))
  (bind _staticmesh (Variables|Default|GetStaticMesh))
  (bind _returnvalue_2 (Transformation|GetWorldLocation _staticmesh))
  (bind (_x _y) (Math|Vector|BreakVector _returnvalue))
  (bind (_x_2 _y_2) (Math|Vector|BreakVector _returnvalue_2))
  (Physics|SetPhysicsLinearVelocity (Variables|Default|GetStaticMesh) (* (Math|Vector|GetUnitDirection(Vector) (Math|Vector|MakeVector _x _y 0.0) (Math|Vector|MakeVector _x_2 _y_2 5e+01)) (* ForceScale 3e+02)) true "None")
  (Class|PrimitiveComponent|SetPhysicsAngularVelocityinDegrees (Variables|Default|GetStaticMesh) (* (Math|Random|RandomUnitVector) 1e+02) true "None"))

(event Custom|SetColour
  (params (Colour :type Linear%20Color%20Structure))
  (bind _returnvalue (Rendering|Material|CreateDynamicMaterialInstance "/Game/Particles/Materials/DiceMaterial.DiceMaterial" :!class /Script/Engine.KismetMaterialLibrary))
  (Rendering|Material|SetVectorParameterValue _returnvalue "CustomColour" Colour :!class /Script/Engine.MaterialInstanceDynamic)
  (Rendering|Material|SetMaterial (Variables|Default|GetStaticMesh) 0 _returnvalue))

(event EventBeginPlay)

(event Collision|EventActorBeginOverlap
  (params (OtherActor :type Actor%20Object%20Reference)))

(event EventTick
  (params (DeltaSeconds :type Float%20%28single-precision%29)))

(fn ConstructionScript)