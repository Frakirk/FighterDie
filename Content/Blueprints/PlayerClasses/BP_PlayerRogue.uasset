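; Rogue player class with two abilities, Smoke Bomb and Blade Flurry, each gated by a DoOnce that resets after a delay.
; Smoke Bomb teleports along the ability direction and high up, then sweeps down in small steps to settle on a surface, spawning smoke at both ends.
; Blade Flurry runs a timeline that scales walk speed under boosted acceleration and spawns slash actors ahead on event keys.
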(event EventBeginPlay
  (|CallParentFunction) ; This node is disabled and will not be called.\nDrag off pins to build functionality.
)

(event Collision|EventActorBeginOverlap
  (params (OtherActor :type Actor%20Object%20Reference))
  (|CallParentFunction OtherActor) ; This node is disabled and will not be called.\nDrag off pins to build functionality.
)

(event EventTick
  (params (DeltaSeconds :type Float%20%28single-precision%29)))

(event Custom|InputAPress
  (bind _self self)
  (bind _self_2 self)
  (Math|Float|CompareFloat (.z (Transformation|GetActorLocation)) -1e+03
    (:>
      _)
    (:==
      _))
  (Utilities|FlowControl|DoOnce false
    (:Completed
      (Audio|PlaySoundatLocation "/Game/Sound/Effects/RogueSmokeBomb.RogueSmokeBomb" (Transformation|GetActorLocation) "0, 0, 0" 1.0 (Math|Random|RandomFloatinRange 0.9 1.1))
      (Game|SpawnActorfromClass "/Game/Blueprints/Smokebomb.Smokebomb_C" (Transformation|GetActorTransform) "Undefined" _self_2 _self_2)
      (bind _direction (CallFunction|GetAbilityDirection))
      (Transformation|SetActorLocation (+ (+ (* _direction 3e+02) (Transformation|GetActorLocation)) "0, 0,5000.000000") false false)
      (CallFunction|TeleportDown)
      (Game|SpawnActorfromClass "/Game/Blueprints/Smokebomb_Arrive.Smokebomb_Arrive_C" (Transformation|GetActorTransform) "Undefined" _self _self)
      (Utilities|FlowControl|Delay 1.0)
      (CallFunction|ResetSmokeBombCooldown))))

(event Custom|ResetSmokeBombCooldown
  (bind _self self)
  (bind _self_2 self)
  (Utilities|FlowControl|DoOnce false) ; enters at Reset
)

(event Custom|TeleportDown
  (Math|Integer|CompareInt (Variables|Default|GetTeleportDownCounter) 500 :!label _label
    (:>
      _)
    (:==
      _)
    (:<
      (Transformation|SetActorLocation (+ (Transformation|GetActorLocation) "0, 0,-10.000000") true false)
      (Math|Integer|IncrementInt (Variables|Default|GetTeleportDownCounter)
        (:%20%20
          (goto _label)))))
  (Variables|Default|SetTeleportDownCounter 0))

(event Custom|InputXPress
  (bind _returnvalue (Transformation|GetActorTransform))
  (bind _self self)
  (Utilities|FlowControl|DoOnce false
    (:Completed
      (Variables|/Script/Engine.CharacterMovementComponent|SetMaxAcceleration (Variables|Character|GetCharacterMovement) 1e+04)
      (Audio|PlaySoundatLocation "/Game/Sound/Effects/RogueBladeFlurry.RogueBladeFlurry" (Transformation|GetActorLocation))
      (bind _movespeed (Timeline|FlurryTimeline PlayFromStart)
        (:Update
          (Variables|/Script/Engine.CharacterMovementComponent|SetMaxWalkSpeed (Variables|Character|GetCharacterMovement) (* (Variables|Default|GetBaseMoveSpeed) _movespeed)))
        (:Finished
          (Variables|/Script/Engine.CharacterMovementComponent|SetMaxWalkSpeed (Variables|Character|GetCharacterMovement) (Variables|Default|GetBaseMoveSpeed))
          (Variables|/Script/Engine.CharacterMovementComponent|SetMaxAcceleration (Variables|Character|GetCharacterMovement) 2048.0)
          (Utilities|FlowControl|Delay 5.0)
          (CallFunction|ResetBladeFlurryCooldown))
        (:Slashes
          (Game|SpawnActorfromClass "/Game/Blueprints/BP_BladeFlurry.BP_BladeFlurry_C" (Math|Transform|MakeTransform (+ (* (Transformation|GetActorForwardVector) 5e+01) (.location _returnvalue)) (.rotation _returnvalue) (.scale _returnvalue)) "Undefined" _self _self))))))

(event Custom|ResetBladeFlurryCooldown
  (bind _returnvalue (Transformation|GetActorTransform))
  (bind _self self)
  (Utilities|FlowControl|DoOnce false) ; enters at Reset
)

(fn ConstructionScript
  (|CallParentFunction))