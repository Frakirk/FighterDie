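; Paladin player character with a steerable charge on input A and a shield on input X, each gated by a cooldown and glow orb.
; Charge boosts movement along a smoothed aim direction, with timeline events firing randomised step sounds and spawning shockwaves.
; Shield spawns a shield actor, brakes velocity and adds half again to any Damage increase while its timeline runs.
; SetColour tints the mesh, shield and hammer through a dynamic material, and spawned actors receive that colour.
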(event Custom|SetColour
  (params (Colour :type Linear%20Color%20Structure))
  (bind _output_get (Variables|Default|SetColour Colour))
  (bind _returnvalue (Rendering|Material|CreateDynamicMaterialInstance "/Game/StarterContent/Materials/M_Basic_Wall.M_Basic_Wall" :!class /Script/Engine.KismetMaterialLibrary))
  (Rendering|Material|SetVectorParameterValue _returnvalue "CustomColour" _output_get :!class /Script/Engine.MaterialInstanceDynamic)
  (Rendering|Material|SetMaterial (Variables|Character|GetMesh) 0 _returnvalue)
  (Rendering|Material|SetMaterial (Variables|Default|Getclinkz_shield) 0 _returnvalue)
  (Rendering|Material|SetMaterial (Variables|Default|Getclinkz_hammer) 0 _returnvalue))

(event EventBeginPlay
  (|CallParentFunction) ; This node is disabled and will not be called.\nDrag off pins to build functionality.
)

(event Collision|EventActorBeginOverlap
  (params (OtherActor :type Actor%20Object%20Reference))
  (|CallParentFunction OtherActor) ; This node is disabled and will not be called.\nDrag off pins to build functionality.
)

(event EventTick
  (params (DeltaSeconds :type Float%20%28single-precision%29)))

(event Custom|PaladinChargeStepSound
  (bind _returnvalue (Math|Random|RandomFloatinRange 0.9 1.1))
  (bind _charge_volume (Variables|Default|GetCharge%20Volume))
  (switch int (Math|Random|RandomIntegerinRange 0 4)
    (:0
      (Audio|PlaySound2D "/Game/Sound/Effects/PaladinStep1.PaladinStep1" _charge_volume _returnvalue))
    (:1
      (Audio|PlaySound2D "/Game/Sound/Effects/PaladinStep2.PaladinStep2" _charge_volume _returnvalue))
    (:2
      (Audio|PlaySound2D "/Game/Sound/Effects/PaladinStep3.PaladinStep3" _charge_volume _returnvalue))
    (:3
      (Audio|PlaySound2D "/Game/Sound/Effects/PaladinStep4.PaladinStep4" _charge_volume _returnvalue))
    (:4
      (Audio|PlaySound2D "/Game/Sound/Effects/PaladinStep5.PaladinStep5" _charge_volume _returnvalue))))

(event Custom|InputAPress
  (bind _charactermovement (Variables|Character|GetCharacterMovement))
  (bind _charactermovement_2 (Variables|Character|GetCharacterMovement))
  (Utilities|FlowControl|DoOnce false
    (:Completed
      (Rendering|ToggleVisibility (Variables|Default|GetGlowOrbA) false)
      (bind _direction (CallFunction|GetAbilityDirection))
      (Variables|Default|SetStoredDirection _direction)
      (Variables|Default|SetMovementDisabled true)
      (Variables|/Script/Engine.CharacterMovementComponent|SetMaxWalkSpeed _charactermovement_2 1e+03)
      (Variables|/Script/Engine.CharacterMovementComponent|SetMaxAcceleration _charactermovement_2 5096.0)
      (Variables|/Script/Engine.CharacterMovementComponent|SetAirControl _charactermovement_2 5.0)
      (Timeline|ChargeTimeline PlayFromStart
        (:Update
          (bind _direction_2 (CallFunction|GetAbilityDirection))
          (bind _output_get (Variables|Default|SetStoredDirection (Math|Vector|Normalize (Math|Vector|Lerp(Vector) (Variables|Default|GetStoredDirection) _direction_2 (* (Utilities|Time|GetWorldDeltaSeconds) 3.0)))))
          (Pawn|Input|AddMovementInput _output_get 1.0 false))
        (:Finished
          (Variables|Default|SetMovementDisabled false)
          (Variables|/Script/Engine.CharacterMovementComponent|SetMaxWalkSpeed _charactermovement 4e+02)
          (Variables|/Script/Engine.CharacterMovementComponent|SetMaxAcceleration _charactermovement 2048.0)
          (Variables|/Script/Engine.CharacterMovementComponent|SetAirControl _charactermovement 0.25)
          (Utilities|FlowControl|Delay 2.0)
          (CallFunction|ResetChargeCooldown))
        (:ChargeEvent
          (CallFunction|CHARGEBLUEPRINT))
        (:Charge%20Step
          (CallFunction|PaladinChargeStepSound))))))

(event Custom|ResetChargeCooldown
  (bind _charactermovement (Variables|Character|GetCharacterMovement))
  (bind _charactermovement_2 (Variables|Character|GetCharacterMovement))
  (Rendering|ToggleVisibility (Variables|Default|GetGlowOrbA) false)
  (Utilities|FlowControl|DoOnce false) ; enters at Reset
)

(event Custom|CHARGEBLUEPRINT
  (bind _returnvalue (Transformation|GetActorTransform))
  (bind _self self)
  (bind _returnvalue_2 (Game|SpawnActorfromClass "/Game/Blueprints/BP_ChargeShockwave.BP_ChargeShockwave_C" (Math|Transform|MakeTransform (+ (.location _returnvalue) (* (Variables|Default|GetStoredDirection) 2e+02)) (.rotation _returnvalue) "1,1,1") "Undefined" _self _self))
  (Variables|/Game/Blueprints/BP_Shockwave.BP_Shockwave_C|SetTargetScale _returnvalue_2 4.0)
  (Variables|/Game/Blueprints/BP_Shockwave.BP_Shockwave_C|SetPowerLevel _returnvalue_2 1)
  (Default|SetColour _returnvalue_2 (Variables|Default|GetColour)))

(event Custom|InputXPress
  (bind _returnvalue (Transformation|GetActorTransform))
  (bind _self self)
  (Utilities|FlowControl|DoOnce false
    (:Completed
      (Rendering|ToggleVisibility (Variables|Default|GetGlowOrbX) false)
      (Audio|PlaySoundatLocation "/Game/Sound/Effects/PaladinShield.PaladinShield" (Transformation|GetActorLocation) "0, 0, 0" 1.0 (Math|Random|RandomFloatinRange 0.9 1.1))
      (Variables|Default|SetStoredDamage (Variables|Default|GetDamage))
      (bind _returnvalue_2 (Game|SpawnActorfromClass "/Game/Blueprints/BP_PaladinShield.BP_PaladinShield_C" (Math|Transform|MakeTransform (+ (.location _returnvalue) "0.000000,0.000000,200.000000") (.rotation _returnvalue) (.scale _returnvalue)) "Undefined" _self _self))
      (Default|SetColour _returnvalue_2 (Variables|Default|GetColour))
      (Timeline|Shield%20Timeline PlayFromStart
        (:Update
          (Variables|/Script/Engine.MovementComponent|SetVelocity (Variables|Character|GetCharacterMovement) (Math|Vector|Lerp(Vector) (Transformation|GetVelocity) "0, 0, 0" (* (Utilities|Time|GetWorldDeltaSeconds) 15.0)))
          (Math|Float|CompareFloat (- (Variables|Default|GetDamage) (Variables|Default|GetStoredDamage)) 0.0
            (:>
              (Variables|Default|SetDamage (Math|Conversions|ToFloat(Integer) (Math|Float|Round (+ (Variables|Default|GetDamage) (* (- (Variables|Default|GetDamage) (Variables|Default|GetStoredDamage)) 0.5))))))
            (:==
              _)
            (:<
              _))
          (Variables|Default|SetStoredDamage (Math|Conversions|ToFloat(Integer) (Math|Float|Round (Variables|Default|GetDamage)))))
        (:Finished
          (Utilities|FlowControl|Delay 4.0)
          (CallFunction|ShieldCooldown))))))

(event Custom|ShieldCooldown
  (bind _returnvalue (Transformation|GetActorTransform))
  (bind _self self)
  (Rendering|ToggleVisibility (Variables|Default|GetGlowOrbX) false)
  (Utilities|FlowControl|DoOnce false) ; enters at Reset
)

(fn ConstructionScript
  (|CallParentFunction))