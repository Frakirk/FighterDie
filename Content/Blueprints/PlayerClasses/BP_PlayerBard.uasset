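; BP_PlayerBard is the Bard player class, with a tintable mesh, hat and guitar and two cooldown-gated abilities shown by glow orbs.
; X fires a power chord, spawning a BP_BWANG projectile along the ability direction.
; A starts a timeline-driven powerslide that boosts movement, locks control and spawns a shockwave when finished.
; The slide tracks peak speed to detect interruption and jump the timeline.
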(event Custom|SetColour
  (params (Colour :type Linear%20Color%20Structure))
  (bind _output_get (Variables|Default|SetColour Colour))
  (bind _returnvalue (Rendering|Material|CreateDynamicMaterialInstance "/Game/StarterContent/Materials/M_Basic_Wall.M_Basic_Wall" :!class /Script/Engine.KismetMaterialLibrary))
  (Rendering|Material|SetVectorParameterValue _returnvalue "CustomColour" _output_get :!class /Script/Engine.MaterialInstanceDynamic)
  (Rendering|Material|SetMaterial (Variables|Character|GetMesh) 0 _returnvalue)
  (Rendering|Material|SetMaterial (Variables|Default|Getbard_hat) 0 _returnvalue)
  (Rendering|Material|SetMaterial (Variables|Default|Getclinkz_guitar) 0 _returnvalue))

(event EventBeginPlay
  (|CallParentFunction) ; This node is disabled and will not be called.\nDrag off pins to build functionality.
)

(event Collision|EventActorBeginOverlap
  (params (OtherActor :type Actor%20Object%20Reference))
  (|CallParentFunction OtherActor) ; This node is disabled and will not be called.\nDrag off pins to build functionality.
)

(event EventTick
  (params (DeltaSeconds :type Float%20%28single-precision%29)))

(event Custom|ResetChordCooldown
  (bind _self self)
  (Rendering|ToggleVisibility (Variables|Default|GetGlowOrbX) false)
  (Utilities|FlowControl|DoOnce false) ; enters at Reset
)

(event Custom|InputXPress
  (bind _self self)
  (Utilities|FlowControl|DoOnce false
    (:Completed
      (Rendering|ToggleVisibility (Variables|Default|GetGlowOrbX) false)
      (bind _returnvalue (Game|SpawnActorfromClass "/Game/Blueprints/BP_BWANG.BP_BWANG_C" (Transformation|GetActorTransform) "Undefined" _self _self))
      (bind _direction (CallFunction|GetAbilityDirection))
      (Variables|/Game/Blueprints/BP_BWANG.BP_BWANG_C|SetMoveDirection _returnvalue _direction)
      (Variables|/Game/Blueprints/BP_Shockwave.BP_Shockwave_C|SetPowerLevel _returnvalue 2)
      (Audio|PlaySoundatLocation "/Game/Sound/Effects/BardPowerChord.BardPowerChord" (Transformation|GetActorLocation) "0, 0, 0" 0.5 (Math|Random|RandomFloatinRange 0.9 1.1))
      (Utilities|FlowControl|Delay 3.0)
      (CallFunction|ResetChordCooldown))))

(event Custom|InputAPress
  (bind _returnvalue (Transformation|GetVelocity))
  (bind _self self)
  (bind _charactermovement (Variables|Character|GetCharacterMovement))
  (bind _charactermovement_2 (Variables|Character|GetCharacterMovement))
  (bind _returnvalue_2 (Math|Vector|VectorLength _returnvalue))
  (Utilities|FlowControl|DoOnce false
    (:Completed
      (Rendering|ToggleVisibility (Variables|Default|GetGlowOrbA) false)
      (bind _returnvalue_3 (Audio|SpawnSoundatLocation "/Game/Sound/Effects/BardPowerslide.BardPowerslide" (Transformation|GetActorLocation) "0, 0, 0" 1.0 (Math|Random|RandomFloatinRange 1.0 2.0)))
      (Variables|Default|SetPowerslideSoundReference _returnvalue_3)
      (bind _direction (CallFunction|GetAbilityDirection))
      (Variables|Default|SetStoredDirection _direction)
      (Variables|/Script/Engine.CharacterMovementComponent|SetMaxWalkSpeed _charactermovement 5e+03)
      (Variables|/Script/Engine.CharacterMovementComponent|SetMaxAcceleration _charactermovement 1e+04)
      (Variables|/Script/Engine.CharacterMovementComponent|SetAirControl _charactermovement 1e+01)
      (Variables|Default|SetMovementDisabled true)
      (Variables|Default|SetSlideSpeed 0.0)
      (Variables|/Script/Engine.MovementComponent|SetVelocity _charactermovement "0, 0, 0")
      (Timeline|PowerslideTimeline PlayFromStart
        (:Update
          (Pawn|Input|AddMovementInput (Variables|Default|GetStoredDirection) 1.0 false)
          (Math|Float|CompareFloat _returnvalue_2 (Variables|Default|GetSlideSpeed)
            (:>
              (Variables|Default|SetSlideSpeed _returnvalue_2)
              (goto _label Reset))
            (:<
              (Utilities|FlowControl|DoOnce true :!label _label
                (:Completed
                  (CallFunction|StopSlide))))))
        (:Finished
          (Game|SpawnActorfromClass "/Game/Blueprints/BP_PowerslideShockwave.BP_PowerslideShockwave_C" (Transformation|GetActorTransform) "Undefined" _self _self)
          (Variables|/Script/Engine.CharacterMovementComponent|SetMaxWalkSpeed _charactermovement_2 5e+02)
          (Variables|/Script/Engine.CharacterMovementComponent|SetMaxAcceleration _charactermovement_2 2048.0)
          (Variables|/Script/Engine.CharacterMovementComponent|SetAirControl _charactermovement_2 0.25)
          (Variables|Default|SetMovementDisabled false)
          (Variables|/Script/Engine.MovementComponent|SetVelocity (Variables|Character|GetCharacterMovement) (Math|Vector|Lerp(Vector) (Transformation|GetVelocity) "0, 0, 0" 0.75))
          (Utilities|FlowControl|Delay 0.5)
          (Audio|Components|Audio|Stop (Variables|Default|GetPowerslideSoundReference))
          (Utilities|FlowControl|Delay 0.75)
          (CallFunction|ResetPowerslideCooldown))))))

(event Custom|StopSlide
  (bind _returnvalue (Transformation|GetVelocity))
  (bind _self self)
  (bind _charactermovement (Variables|Character|GetCharacterMovement))
  (bind _returnvalue_2 (Math|Vector|VectorLength _returnvalue))
  (Development|PrintString "slide interrupted")
  (Timeline|PowerslideTimeline SetNewTime
    (:Update
      (Pawn|Input|AddMovementInput (Variables|Default|GetStoredDirection) 1.0 false)
      (Math|Float|CompareFloat _returnvalue_2 (Variables|Default|GetSlideSpeed)
        (:>
          (Variables|Default|SetSlideSpeed _returnvalue_2)
          (goto _label Reset))
        (:<
          (Utilities|FlowControl|DoOnce true :!label _label
            (:Completed
              (CallFunction|StopSlide))))))
    (:Finished
      (Game|SpawnActorfromClass "/Game/Blueprints/BP_PowerslideShockwave.BP_PowerslideShockwave_C" (Transformation|GetActorTransform) "Undefined" _self _self)
      (Variables|/Script/Engine.CharacterMovementComponent|SetMaxWalkSpeed _charactermovement 5e+02)
      (Variables|/Script/Engine.CharacterMovementComponent|SetMaxAcceleration _charactermovement 2048.0)
      (Variables|/Script/Engine.CharacterMovementComponent|SetAirControl _charactermovement 0.25)
      (Variables|Default|SetMovementDisabled false)
      (Variables|/Script/Engine.MovementComponent|SetVelocity (Variables|Character|GetCharacterMovement) (Math|Vector|Lerp(Vector) (Transformation|GetVelocity) "0, 0, 0" 0.75))
      (Utilities|FlowControl|Delay 0.5)
      (Audio|Components|Audio|Stop (Variables|Default|GetPowerslideSoundReference))
      (Utilities|FlowControl|Delay 0.75)
      (CallFunction|ResetPowerslideCooldown))))

(event Custom|ResetPowerslideCooldown
  (bind _returnvalue (Transformation|GetVelocity))
  (bind _self self)
  (bind _charactermovement (Variables|Character|GetCharacterMovement))
  (bind _charactermovement_2 (Variables|Character|GetCharacterMovement))
  (bind _returnvalue_2 (Math|Vector|VectorLength _returnvalue))
  (Rendering|ToggleVisibility (Variables|Default|GetGlowOrbA) false)
  (Utilities|FlowControl|DoOnce false) ; enters at Reset
)

(fn ConstructionScript
  (|CallParentFunction))