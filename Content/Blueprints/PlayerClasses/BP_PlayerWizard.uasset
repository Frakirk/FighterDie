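; Wizard player character Blueprint with two abilities: a projectile teleport and a chargeable shockwave.
; A press launches a teleport orb along the input direction; releasing or a timeout moves the wizard to it, with a DoOnce-gated cooldown.
; X plays a timeline that modulates walk speed and accumulates power, then spawns a power-scaled shockwave when finished.
; Releasing X changes the timeline's playback time.
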(event EventBeginPlay)

(event Collision|EventActorBeginOverlap
  (params (OtherActor :type Actor%20Object%20Reference))
  (|CallParentFunction OtherActor) ; This node is disabled and will not be called.\nDrag off pins to build functionality.
)

(event EventTick
  (params (DeltaSeconds :type Float%20%28single-precision%29)))

(event Custom|InputAPress
  (Utilities|FlowControl|DoOnce false
    (:Completed
      (bind _returnvalue (Game|SpawnActorfromClass "/Game/Blueprints/BP_PlayerTeleport.BP_PlayerTeleport_C" (Math|Transform|MakeTransform (+ (Transformation|GetActorLocation) "0, 0,150.000000") "0, 0, 0" "0.500000,0.500000,0.500000") "AdjustIfPossibleButAlwaysSpawn" self 0))
      (Physics|SetPhysicsLinearVelocity (Variables|/Game/Blueprints/BP_PlayerTeleport.BP_PlayerTeleport_C|GetSphere _returnvalue) (* (Math|Vector|Normalize (Math|Vector|MakeVector (Input|AxisValues|GetUp) (Input|AxisValues|GetRight) 0.0)) 1.5e+03) false "None")
      (Utilities|FlowControl|Delay 2.0)
      (CallFunction|ResetTeleportCooldown)
      (CallFunction|TeleportEnd))))

(event Custom|InputARelease
  (CallFunction|TeleportEnd))

(event Custom|ResetTeleportCooldown
  (Utilities|FlowControl|Delay 1.0)
  (Development|PrintString "Teleport Ready")
  (Utilities|FlowControl|DoOnce false) ; enters at Reset
)

(event Custom|TeleportEnd
  (Utilities|IsValid (stale Custom|InputAPress _returnvalue)
    (:Is%20Valid
      (Transformation|SetActorLocation (+ (Transformation|GetActorLocation (stale Custom|InputAPress _returnvalue)) "0, 0,-150.000000") false false)
      (Actor|DestroyActor (stale Custom|InputAPress _returnvalue)))))

(event Custom|InputXPress
  (bind _self self)
  (if (not (Audio|Components|Audio|IsPlaying (Variables|Default|GetAttackTimeLine)))
    (Audio|PlaySoundatLocation "/Game/Sound/Effects/WizardChargeUp.WizardChargeUp" (Transformation|GetActorLocation))
    (Variables|Default|SetShockwavePower 0)
    (bind _maxwalkspeedmod (Timeline|AttackTimeline PlayFromStart)
      (:Update
        (Variables|/Script/Engine.CharacterMovementComponent|SetMaxWalkSpeed (Variables|Character|GetCharacterMovement) (* _maxwalkspeedmod 5e+02)))
      (:Finished
        (Variables|/Script/Engine.CharacterMovementComponent|SetMaxWalkSpeed (Variables|Character|GetCharacterMovement) 5e+02)
        (Math|Integer|CompareInt (Variables|Default|GetShockwavePower)
          (:>
            (bind _returnvalue (Game|SpawnActorfromClass "/Game/Blueprints/BP_PlayerShockwave.BP_PlayerShockwave_C" (Transformation|GetActorTransform) "Undefined" _self _self))
            (Variables|/Game/Blueprints/BP_Shockwave.BP_Shockwave_C|SetPowerLevel _returnvalue (Variables|Default|GetShockwavePower))
            (Variables|/Game/Blueprints/BP_Shockwave.BP_Shockwave_C|SetTargetScale _returnvalue (* (Variables|Default|GetShockwavePower) 5.0)))))
      (:PowerCharge
        (bind _result (Math|Integer|IncrementInt (Variables|Default|GetShockwavePower))
          (:%20%20
            (Development|PrintString (Utilities|String|ToString(Integer) _result))))))))

(event Custom|InputXRelease
  (bind _self self)
  (bind _shockwavepower (Variables|Default|GetShockwavePower))
  (if (Audio|Components|Audio|IsPlaying (Variables|Default|GetAttackTimeLine))
    (bind _maxwalkspeedmod (Timeline|AttackTimeline SetNewTime)
      (:Update
        (Variables|/Script/Engine.CharacterMovementComponent|SetMaxWalkSpeed (Variables|Character|GetCharacterMovement) (* _maxwalkspeedmod 5e+02)))
      (:Finished
        (Variables|/Script/Engine.CharacterMovementComponent|SetMaxWalkSpeed (Variables|Character|GetCharacterMovement) 5e+02)
        (Math|Integer|CompareInt (Variables|Default|GetShockwavePower)
          (:>
            (bind _returnvalue (Game|SpawnActorfromClass "/Game/Blueprints/BP_PlayerShockwave.BP_PlayerShockwave_C" (Transformation|GetActorTransform) "Undefined" _self _self))
            (Variables|/Game/Blueprints/BP_Shockwave.BP_Shockwave_C|SetPowerLevel _returnvalue _shockwavepower)
            (Variables|/Game/Blueprints/BP_Shockwave.BP_Shockwave_C|SetTargetScale _returnvalue (* _shockwavepower 5.0)))))
      (:PowerCharge
        (bind _result (Math|Integer|IncrementInt (Variables|Default|GetShockwavePower))
          (:%20%20
            (Development|PrintString (Utilities|String|ToString(Integer) _result))))))))

(fn ConstructionScript
  (|CallParentFunction))