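; FighterDieGameMode is a game mode that sets up local players and their colours in the Test1 level.
; On BeginPlay it checks the level name, then creates the extra players needed to reach PlayerCount.
; After each creation it gathers all PlayerCharacter actors and applies PlayerColours by array index, so colours follow actor search order rather than player index.
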(event EventBeginPlay
  (bind _returnvalue (Game|GetCurrentLevelName true))
  (if (Utilities|Enum|Equal(Enum) _returnvalue "Test1")
    (for _index (range 2 (Variables|Default|GetPlayer%20count))
      (Class|GameplayStatics|CreatePlayer -1)
      (bind _outactors (Actor|GetAllActorsOfClass "/Game/Blueprints/PlayerCharacter.PlayerCharacter_C"))
      (for (_array_element _array_index) _outactors
        (bind _asplayer_character (Utilities|Casting|CastToPlayerCharacter _array_element))
        (Default|SetColour _asplayer_character (Utilities|Array|Get(acopy) (Variables|Default|GetPlayerColours) _array_index))))))

(event EventTick
  (params (DeltaSeconds :type Float%20%28single-precision%29)))

(fn ConstructionScript)