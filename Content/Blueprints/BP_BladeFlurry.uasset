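; BP_BladeFlurry is a short-lived attack hitbox, apparently for a blade flurry, that affects players and dice.
; BeginPlay runs the parent logic and sets PowerLevel.
; Box overlaps with any actor other than its owner are passed to HitPlayers and HitDice, which are defined outside this file.
; Tick resets the actor's scale and uses a brief Delay before destroying it.
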(event OnComponentBeginOverlap(Box)
  (params (OverlappedComponent :type Primitive%20Component%20Object%20Reference) (OtherActor :type Actor%20Object%20Reference) (OtherComp :type Primitive%20Component%20Object%20Reference) (OtherBodyIndex :type Integer) (bFromSweep :type Boolean) (SweepResult :type Hit%20Result%20Structure%20%28by%20ref%29))
  (if (not (== (Components|GetOwner) OtherActor))
    (CallFunction|HitPlayers OtherActor)
    (CallFunction|HitDice OtherActor)))

(event EventBeginPlay
  (|CallParentFunction)
  (Variables|Default|SetPowerLevel 3))

(event Collision|EventActorBeginOverlap
  (params (OtherActor :type Actor%20Object%20Reference))
  (|CallParentFunction OtherActor) ; This node is disabled and will not be called.\nDrag off pins to build functionality.
)

(event EventTick
  (params (DeltaSeconds :type Float%20%28single-precision%29))
  (Transformation|SetActorScale3D "1.000000,1.000000,1.000000")
  (Utilities|FlowControl|Delay 0.1)
  (Actor|DestroyActor))

(fn ConstructionScript
  (|CallParentFunction))