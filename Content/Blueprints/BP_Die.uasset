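; BP_Die is a physics die that players knock around, taking the colour of the last player to hit it.
; When it settles, it finds the raised face marker, hops, and spawns a BP_Shockwave in that player's colour, scaled by the roll.
; A six also spawns a one-shot bonus die that destroys itself after detonating.
; It registers with BP_GameCamera for tracking and teleports back when it strays too far from the origin.
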(event OnComponentHit(Cube)
  (params (HitComponent :type Primitive%20Component%20Object%20Reference) (OtherActor :type Actor%20Object%20Reference) (OtherComp :type Primitive%20Component%20Object%20Reference) (NormalImpulse :type Vector :default "0, 0, 0") (Hit :type Hit%20Result%20Structure%20%28by%20ref%29))
  (if (not (Variables|Default|GetHasBumpPlayed))
    (bind _asplayer_character (Utilities|Casting|CastToPlayerCharacter OtherActor))
    (CallFunction|Bounce _asplayer_character 1.0)
    (Character|LaunchCharacter _asplayer_character (Math|Vector|MakeVector (.X (Math|Vector|BreakVector (* (Math|Vector|GetUnitDirection(Vector) (Transformation|GetWorldLocation (Variables|Default|GetCube)) (Transformation|GetActorLocation _asplayer_character)) 5e+02))) (.Y (Math|Vector|BreakVector (* (Math|Vector|GetUnitDirection(Vector) (Transformation|GetWorldLocation (Variables|Default|GetCube)) (Transformation|GetActorLocation _asplayer_character)) 5e+02))) 2.5e+02) true true)
    (bind _output_get (Variables|Default|SetTaggingPlayer _asplayer_character))
    (CallFunction|SetColour (Variables|/Game/Blueprints/PlayerCharacter.PlayerCharacter_C|GetColour _output_get))
    (CallFunction|DiceBumpSound)))

(event Custom|Bounce
  (params (OtherActor :type Actor%20Object%20Reference) (ForceScale :type Float%20%28single-precision%29))
  (bind _returnvalue (Transformation|GetActorLocation OtherActor))
  (bind _cube (Variables|Default|GetCube))
  (bind _returnvalue_2 (Transformation|GetWorldLocation _cube))
  (bind (_x _y) (Math|Vector|BreakVector _returnvalue))
  (bind (_x_2 _y_2) (Math|Vector|BreakVector _returnvalue_2))
  (Physics|SetPhysicsLinearVelocity (Variables|Default|GetCube) (* (Math|Vector|GetUnitDirection(Vector) (Math|Vector|MakeVector _x _y 0.0) (Math|Vector|MakeVector _x_2 _y_2 5e+01)) (* ForceScale 3e+02)) true "None")
  (Class|PrimitiveComponent|SetPhysicsAngularVelocityinDegrees (Variables|Default|GetCube) (* (Math|Random|RandomUnitVector) 1e+02) true "None"))

(event Custom|SetColour
  (params (Colour :type Linear%20Color%20Structure))
  (bind _returnvalue (Rendering|Material|CreateDynamicMaterialInstance "/Game/Particles/Materials/DiceMaterial.DiceMaterial" :!class /Script/Engine.KismetMaterialLibrary))
  (Rendering|Material|SetVectorParameterValue _returnvalue "CustomColour" Colour :!class /Script/Engine.MaterialInstanceDynamic)
  (Rendering|Material|SetMaterial (Variables|Default|GetCube) 0 _returnvalue))

(event Custom|DiceExplosionSound
  (switch int (Math|Random|RandomIntegerinRange 0 3)
    (:0
      (Audio|PlaySound2D "/Game/Sound/Effects/Explosion1.Explosion1"))
    (:1
      (Audio|PlaySound2D "/Game/Sound/Effects/Explosion2.Explosion2"))
    (:2
      (Audio|PlaySound2D "/Game/Sound/Effects/Explosion3.Explosion3"))
    (:3
      (Audio|PlaySound2D "/Game/Sound/Effects/Explosion4.Explosion4"))))

(event Custom|ResetLocation
  (bind _returnvalue (Transformation|GetVelocity))
  (bind (_x _y) (Math|Vector|BreakVector _returnvalue))
  (Transformation|SetActorLocation "0, 0,380.000000" false false)
  (Physics|SetPhysicsLinearVelocity (Variables|Default|GetCube) (Math|Vector|MakeVector _x _y 0.0) false "None")
  (Class|PrimitiveComponent|SetPhysicsAngularVelocityinDegrees (Variables|Default|GetCube) (* (Math|Random|RandomUnitVector) 1e+03) false "None"))

(event Custom|DiceBumpSound
  (bind _returnvalue (Transformation|GetActorLocation))
  (bind _returnvalue_2 (Math|Random|RandomFloatinRange 0.8 1.2))
  (bind _volumelevel (Variables|Default|GetVolumeLevel))
  (switch int (Math|Random|RandomIntegerinRange 0 3)
    (:0
      (Audio|SpawnSoundatLocation "/Game/Sound/Effects/PaladinStep1.PaladinStep1" _returnvalue "0, 0, 0" _volumelevel _returnvalue_2 _returnvalue_2))
    (:1
      (Audio|SpawnSoundatLocation "/Game/Sound/Effects/PaladinStep1.PaladinStep1" _returnvalue "0, 0, 0" _volumelevel _returnvalue_2))
    (:2
      (Audio|SpawnSoundatLocation "/Game/Sound/Effects/PaladinStep1.PaladinStep1" _returnvalue "0, 0, 0" _volumelevel _returnvalue_2))
    (:3
      (Audio|SpawnSoundatLocation "/Game/Sound/Effects/PaladinStep1.PaladinStep1" _returnvalue "0, 0, 0" _volumelevel _returnvalue_2)))
  (Variables|Default|SetHasBumpPlayed true)
  (Utilities|FlowControl|Delay 0.1)
  (Variables|Default|SetHasBumpPlayed false))

(event EventBeginPlay
  (bind _outactors (Actor|GetAllActorsOfClass "/Game/Blueprints/BP_GameCamera.BP_GameCamera_C"))
  (Utilities|Array|AddUnique (Variables|/Game/Blueprints/BP_GameCamera.BP_GameCamera_C|GetTrackedObjects (Utilities|Array|Get(acopy) _outactors)) self)
  (CallFunction|SetColour "(R=1.000000,G=1.000000,B=1.000000,A=1.000000)"))

(event EventTick
  (params (DeltaSeconds :type Float%20%28single-precision%29))
  (bind _returnvalue (Transformation|GetActorLocation))
  (bind (_x _y) (Math|Vector|BreakVector _returnvalue))
  (bind _returnvalue_2 (* _y -0.9))
  (bind _returnvalue_3 (* _x -0.9))
  (bind _returnvalue_4 (Math|Vector|MakeVector _returnvalue_3 _returnvalue_2 5e+02))
  (Math|Float|CompareFloat (Math|Vector|VectorLength _returnvalue) 2e+03
    (:>
      (Transformation|SetActorLocation _returnvalue_4 false false)
      (Physics|SetPhysicsLinearVelocity (Variables|Default|GetCube) _returnvalue_4 false "None"))
    (:==
      _)
    (:<
      _))
  (bind _returnvalue_5 (Physics|GetPhysicsLinearVelocity (Variables|Default|GetCube) "None"))
  (Math|Float|CompareFloat (Math|Vector|VectorLength _returnvalue_5) 0.01
    (:>
      (goto _label Reset))
    (:<
      (Utilities|FlowControl|DoOnce true :!label _label
        (:Completed
          (Utilities|IsValid (Variables|Default|GetTaggingPlayer)
            (:Is%20Valid
              (bind _result (CallFunction|GetDieResult))
              (Math|Integer|CompareInt _result 6
                (:==
                  (bind _returnvalue_6 (Game|SpawnActorfromClass "BP_Die_C" (Math|Transform|MakeTransform (+ (Transformation|GetActorLocation) "0, 0,100.000000") "35.000000,380.000000,45.000000" "0.500000,0.500000,0.500000") "AdjustIfPossibleButAlwaysSpawn" 0 0))
                  (bind _output_get (Variables|BP_Die_C|SetTaggingPlayer _returnvalue_6 (Variables|Default|GetTaggingPlayer)))
                  (CallFunction|SetColour _returnvalue_6 (Variables|/Game/Blueprints/PlayerCharacter.PlayerCharacter_C|GetColour _output_get))
                  (Variables|BP_Die_C|SetOneShot _returnvalue_6 true))
                (:<
                  _))
              (bind _returnvalue_7 (Game|SpawnActorfromClass "/Game/Blueprints/BP_Shockwave.BP_Shockwave_C" (Math|Conversions|ToTransform(Vector) (Transformation|GetWorldLocation (Variables|Default|GetCube))) "AlwaysSpawn" 0 0))
              (Default|SetColour _returnvalue_7 (Variables|/Game/Blueprints/PlayerCharacter.PlayerCharacter_C|GetColour (Variables|Default|GetTaggingPlayer)))
              (Variables|/Game/Blueprints/BP_Shockwave.BP_Shockwave_C|SetTaggingPlayer _returnvalue_7 (Variables|Default|GetTaggingPlayer))
              (bind _output_get_2 (Variables|/Game/Blueprints/BP_Shockwave.BP_Shockwave_C|SetPowerLevel _returnvalue_7 _result))
              (Variables|/Game/Blueprints/BP_Shockwave.BP_Shockwave_C|SetTargetScale _returnvalue_7 (+ 4e+01 (* _output_get_2 1e+01)))
              (Variables|Default|SetTaggingPlayer 0)
              (CallFunction|SetColour "(R=1.000000,G=1.000000,B=1.000000,A=1.000000)")
              (CallFunction|DiceExplosionSound)
              (if (Variables|Default|GetOneShot)
                (Actor|DestroyActor)))))))))

(event EventDestroyed
  (bind _outactors (Actor|GetAllActorsOfClass "/Game/Blueprints/BP_GameCamera.BP_GameCamera_C"))
  (Utilities|Array|RemoveItem (Variables|/Game/Blueprints/BP_GameCamera.BP_GameCamera_C|GetTrackedObjects (Utilities|Array|Get(acopy) _outactors)) self))

(fn ConstructionScript
  (Variables|Default|SetDieFaces (Utilities|Array|MakeArray (Variables|Default|GetScene1) (Variables|Default|GetScene2) (Variables|Default|GetScene3) (Variables|Default|GetScene4) (Variables|Default|GetScene5) (Variables|Default|GetScene6))))

(fn GetDieResult
  (bind _returnvalue (Math|Random|RandomUnitVector))
  (bind _returnvalue_2 (* _returnvalue 1e+03))
  (bind (_x _y) (Math|Vector|BreakVector _returnvalue_2))
  (for (_array_element _array_index) (Variables|Default|GetDieFaces)
    (Math|Float|CompareFloat (.Z (Math|Vector|BreakVector (Transformation|GetWorldLocation _array_element))) (+ (.Z (Math|Vector|BreakVector (Transformation|GetWorldLocation (Variables|Default|GetCube)))) 45.0)
      (:>
        (Math|Integer|CompareInt (+ _array_index 1) 6
          (:==
            _)
          (:<
            _))
        (Physics|SetPhysicsLinearVelocity (Variables|Default|GetCube) (Math|Vector|MakeVector (.X (Math|Vector|BreakVector (* (Math|Vector|Normalize (Math|Vector|MakeVector _x _y 0.0)) (* (+ _array_index 1) 1.5e+02)))) (.Y (Math|Vector|BreakVector (* (Math|Vector|Normalize (Math|Vector|MakeVector _x _y 0.0)) (* (+ _array_index 1) 1.5e+02)))) 5e+02) true "None")
        (Class|PrimitiveComponent|SetPhysicsAngularVelocityinDegrees (Variables|Default|GetCube) (* (Math|Random|RandomUnitVector) 2e+02) true "None")
        (return (+ _array_index 1)))))
  (return 0))