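; Spinning circle actor, apparently a platform, that rotates around its yaw axis through a timeline.
; BeginPlay uses the timeline's Set New Time input, with a random value feeding New Time to offset the starting phase.
; Tick keeps the timeline playing, its Angle track sets actor yaw, and a custom Restart event replays it from the start on finish.
; An older incrementing PlatformRotation wrap-around remains disconnected.
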(event Custom|Restart
  (bind _angle (Timeline|SpinnyTimeline PlayFromStart)
    (:Update
      (Transformation|SetActorRotation (Math|Rotator|MakeRotator 0.0 0.0 _angle)))
    (:Finished
      (CallFunction|Restart))))

(event EventBeginPlay
  (bind _angle (Timeline|SpinnyTimeline SetNewTime)
    (:Update
      (Transformation|SetActorRotation (Math|Rotator|MakeRotator 0.0 0.0 _angle)))
    (:Finished
      (CallFunction|Restart))))

(event Collision|EventActorBeginOverlap
  (params (OtherActor :type Actor%20Object%20Reference)))

(event EventTick
  (params (DeltaSeconds :type Float%20%28single-precision%29))
  (bind _angle (Timeline|SpinnyTimeline Play)
    (:Update
      (Transformation|SetActorRotation (Math|Rotator|MakeRotator 0.0 0.0 _angle)))
    (:Finished
      (CallFunction|Restart))))

(fn ConstructionScript)