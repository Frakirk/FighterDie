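; BP_PaladinShield is the Paladin's shield actor, a temporary effect that surrounds its Instigator.
; It doubles its scale on spawn, then snaps to the Instigator's location every tick.
; Opacity is driven by the remaining fraction of its lifespan.
; Sphere overlaps pass the other actor to HitPlayers and HitDice, which are defined outside these graphs.
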(event OnComponentBeginOverlap(Sphere)
  (params (OverlappedComponent :type Primitive%20Component%20Object%20Reference) (OtherActor :type Actor%20Object%20Reference) (OtherComp :type Primitive%20Component%20Object%20Reference) (OtherBodyIndex :type Integer) (bFromSweep :type Boolean) (SweepResult :type Hit%20Result%20Structure%20%28by%20ref%29))
  (CallFunction|HitPlayers OtherActor)
  (CallFunction|HitDice OtherActor))

(event EventBeginPlay
  (|CallParentFunction)
  (Transformation|SetActorScale3D "2.000000,2.000000,2.000000"))

(event Collision|EventActorBeginOverlap
  (params (OtherActor :type Actor%20Object%20Reference))
  (|CallParentFunction OtherActor) ; This node is disabled and will not be called.\nDrag off pins to build functionality.
)

(event EventTick
  (params (DeltaSeconds :type Float%20%28single-precision%29))
  (Transformation|SetActorLocation (Transformation|GetActorLocation (Variables|Default|GetInstigator)) false false)
  (CallFunction|SetOpacity (/ (Actor|GetLifeSpan) (Variables|Default|GetInitialLifeSpan)) 0.05))

(fn ConstructionScript
  (|CallParentFunction))