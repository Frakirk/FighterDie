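; Expanding shockwave that damages and launches players, and bounces dice.
; Tick grows it toward TargetScale and fades its Instigator-coloured bubble material over its lifespan.
; Sphere overlaps affect each target once, sparing owner and tagging player, and re-tag dice to the owner.
; Knockback radiates from the Instigator or shockwave, scaling with power and accumulated damage and weakening with remaining lifespan; damage falloff is optional.
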(event OnComponentBeginOverlap(Sphere)
  (params (OverlappedComponent :type Primitive%20Component%20Object%20Reference) (OtherActor :type Actor%20Object%20Reference) (OtherComp :type Primitive%20Component%20Object%20Reference) (OtherBodyIndex :type Integer) (bFromSweep :type Boolean) (SweepResult :type Hit%20Result%20Structure%20%28by%20ref%29))
  (CallFunction|HitPlayers OtherActor)
  (CallFunction|HitDice OtherActor))

(event Custom|HitPlayers
  (params (Other%20Actor :type Actor%20Object%20Reference))
  (if (!= Other%20Actor (Components|GetOwner))
    (bind _asplayer_character (Utilities|Casting|CastToPlayerCharacter Other%20Actor))
    (Math|Integer|CompareInt (Utilities|Array|FindItem (Variables|Default|GetPlayersHit) _asplayer_character) -1
      (:==
        (Utilities|Array|AddUnique (Variables|Default|GetPlayersHit) _asplayer_character)
        (if (!= (Variables|Default|GetTaggingPlayer) _asplayer_character)
          (Utilities|ApplyDamage _asplayer_character (Variables|Default|GetNoFalloff)
            (:%20%20
              (if (Variables|Default|GetInstigatorIsOrigin)
                (bind _velocity (CallFunction|CalculateLaunchVelocity false (Variables|Actor|GetInstigator) _asplayer_character))
                (Character|LaunchCharacter _asplayer_character _velocity false false)
                (else
                  (bind _velocity_2 (CallFunction|CalculateLaunchVelocity false self _asplayer_character))
                  (Character|LaunchCharacter _asplayer_character _velocity_2 false false))))))))))

(event Custom|SetOpacity
  (params (Alpha :type Float%20%28single-precision%29) (Coefficient :type Float%20%28single-precision%29))
  (bind _dynamicmaterialref (Variables|Default|GetDynamicMaterialRef))
  (Rendering|Material|SetScalarParameterValue _dynamicmaterialref "CustomAlpha" (* Alpha Coefficient) :!class /Script/Engine.MaterialInstanceDynamic)
  (Rendering|Material|SetMaterial (Variables|Default|GetSphere1) 0 _dynamicmaterialref))

(event Custom|SetColour
  (params (Colour :type Linear%20Color%20Structure))
  (bind _dynamicmaterialref (Variables|Default|GetDynamicMaterialRef))
  (Rendering|Material|SetVectorParameterValue _dynamicmaterialref "CustomColour" (* Colour 1e+02) :!class /Script/Engine.MaterialInstanceDynamic)
  (Rendering|Material|SetMaterial (Variables|Default|GetSphere1) 0 _dynamicmaterialref))

(event Custom|Hit%20Dice
  (params (Other%20Actor :type Actor%20Object%20Reference))
  (bind _returnvalue (Components|GetOwner))
  (bind _powerlevel (Variables|Default|GetPowerLevel))
  (bind _asbp_die (Utilities|Casting|CastToBP_Die Other%20Actor))
  (Math|Integer|CompareInt (Utilities|Array|FindItem (Variables|Default|GetDiceHit) _asbp_die) -1
    (:==
      (Utilities|Array|AddUnique (Variables|Default|GetDiceHit) _asbp_die)
      (if (Variables|Default|GetInstigatorIsOrigin)
        (Default|Bounce _asbp_die (Variables|Actor|GetInstigator) (Math|Conversions|ToFloat(Integer) _powerlevel))
        (else
          (Default|Bounce _asbp_die self (Math|Conversions|ToFloat(Integer) _powerlevel))))
      (Utilities|IsValid _returnvalue
        (:Is%20Valid
          (bind _asplayer_character (Utilities|Casting|CastToPlayerCharacter _returnvalue))
          (Variables|/Game/Blueprints/BP_Die.BP_Die_C|SetTaggingPlayer _asbp_die _asplayer_character)
          (Default|SetColour _asbp_die (Variables|/Game/Blueprints/PlayerCharacter.PlayerCharacter_C|GetColour _asplayer_character)))))))

(event EventBeginPlay
  (bind _returnvalue (Rendering|Material|CreateDynamicMaterialInstance "/Game/Particles/Materials/Bubble.Bubble" :!class /Script/Engine.KismetMaterialLibrary))
  (Variables|Default|SetDynamicMaterialRef _returnvalue)
  (bind _asplayer_character (Utilities|Casting|CastToPlayerCharacter (Variables|Actor|GetInstigator)))
  (CallFunction|SetColour (Variables|/Game/Blueprints/PlayerCharacter.PlayerCharacter_C|GetColour _asplayer_character)))

(event Collision|EventActorBeginOverlap
  (params (OtherActor :type Actor%20Object%20Reference)))

(event EventTick
  (params (DeltaSeconds :type Float%20%28single-precision%29))
  (Transformation|SetActorScale3D (Math|Vector|Lerp(Vector) (Transformation|GetActorScale3D) (Math|Conversions|ToVector(Float) (Variables|Default|GetTargetScale)) DeltaSeconds))
  (CallFunction|SetOpacity (/ (Actor|GetLifeSpan) (Variables|Actor|GetInitialLifeSpan)) 0.01))

(fn ConstructionScript)

(fn CalculateLaunchVelocity
  (params (NoFalloff :type Boolean) (OriginActor :type Actor%20Object%20Reference) (PawnRef :type Player%20Character%20Object%20Reference))
  (bind _returnvalue (Transformation|GetActorLocation OriginActor))
  (bind _returnvalue_2 (Transformation|GetActorLocation PawnRef))
  (bind _powerlevel (Variables|Default|GetPowerLevel))
  (bind _damage (Variables|/Game/Blueprints/PlayerCharacter.PlayerCharacter_C|GetDamage PawnRef))
  (bind _powerlevel_2 (Variables|Default|GetPowerLevel))
  (bind _returnvalue_3 (- _returnvalue_2 _returnvalue))
  (bind _returnvalue_4 (+ _damage 1e+02))
  (bind _returnvalue_5 (+ _damage 4e+02))
  (bind _returnvalue_6 (* _powerlevel _returnvalue_4))
  (bind _returnvalue_7 (* _powerlevel_2 _returnvalue_5))
  (bind _returnvalue_8 (Math|Vector|Normalize _returnvalue_3))
  (bind _returnvalue_9 (* _returnvalue_8 _returnvalue_7))
  (bind (_x _y) (Math|Vector|BreakVector _returnvalue_9))
  (bind _returnvalue_10 (Math|Vector|MakeVector _x _y _returnvalue_6))
  (if NoFalloff
    (return _returnvalue_10)
    (else
      (return (* _returnvalue_10 (/ (Actor|GetLifeSpan) (Variables|Actor|GetInitialLifeSpan)))))))