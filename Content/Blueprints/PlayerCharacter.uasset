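; Player character that moves on fixed world axes, registers with BP_GameCamera for tracking and colours its mesh through a dynamic material.
; Attack runs a timeline that modulates walk speed, then restores it, spawns a shockwave and raises the character's Damage variable.
; Teleport lobs a physics-driven BP_PlayerTeleport actor upward along the movement input, gated by a DoOnce that resets after a short cooldown.
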(event Custom|ResetTeleportCooldown
  (Utilities|FlowControl|DoOnce false) ; enters at Reset
)

(event Custom|SetColour
  (params (Colour :type Linear%20Color%20Structure))
  (bind _output_get (Variables|Default|SetColour Colour))
  (bind _returnvalue (Rendering|Material|CreateDynamicMaterialInstance "/Game/StarterContent/Materials/M_Basic_Wall.M_Basic_Wall" :!class /Script/Engine.KismetMaterialLibrary))
  (Rendering|Material|SetVectorParameterValue _returnvalue "CustomColour" _output_get :!class /Script/Engine.MaterialInstanceDynamic)
  (Rendering|Material|SetMaterial (Variables|Default|GetStaticMesh) 0 _returnvalue))

(event EventBeginPlay
  (bind _outactors (Actor|GetAllActorsOfClass "/Game/Blueprints/BP_GameCamera.BP_GameCamera_C"))
  (Utilities|Array|AddUnique (Variables|/Game/Blueprints/BP_GameCamera.BP_GameCamera_C|GetTrackedObjects (Utilities|Array|Get(acopy) _outactors)) self)
  (CallFunction|SetColour "(R=0.000000,G=0.250000,B=1.000000,A=1.000000)"))

(event Collision|EventActorBeginOverlap
  (params (OtherActor :type Actor%20Object%20Reference)))

(event EventTick
  (params (DeltaSeconds :type Float%20%28single-precision%29)))

(event Input|ActionEvents|InputActionAttack
  (params (Key :type Key%20Structure))
  (bind _self self)
  (:Pressed
    (if (not (Audio|Components|Audio|IsPlaying (Variables|Default|GetAttackTimeLine)))
      (bind _maxwalkspeedmod (Timeline|AttackTimeLine PlayFromStart)
        (:Update
          (Variables|/Script/Engine.CharacterMovementComponent|SetMaxWalkSpeed (Variables|Character|GetCharacterMovement) (* _maxwalkspeedmod 3e+02)))
        (:Finished
          (Variables|/Script/Engine.CharacterMovementComponent|SetMaxWalkSpeed (Variables|Character|GetCharacterMovement) 3e+02)
          (Game|SpawnActorfromClass "/Game/Blueprints/BP_PlayerShockwave.BP_PlayerShockwave_C" (Transformation|GetActorTransform) "Undefined" _self _self)
          (Variables|Default|SetDamage (+ (Variables|Default|GetDamage) 12.0)))))))

(event Input|ActionEvents|InputActionTeleport
  (params (Key :type Key%20Structure))
  (:Pressed
    (Utilities|FlowControl|DoOnce false
      (:Completed
        (bind _returnvalue (Game|SpawnActorfromClass "/Game/Blueprints/BP_PlayerTeleport.BP_PlayerTeleport_C" (Math|Transform|MakeTransform (+ (Transformation|GetActorLocation) "0, 0,150.000000") "0, 0, 0" "0.500000,0.500000,0.500000") "AdjustIfPossibleButAlwaysSpawn" self 0))
        (Physics|SetPhysicsLinearVelocity (Variables|/Game/Blueprints/BP_PlayerTeleport.BP_PlayerTeleport_C|GetSphere _returnvalue) (* (Math|Vector|Normalize (Math|Vector|MakeVector (Input|AxisValues|GetUp) (Input|AxisValues|GetRight) 1.0)) 1.5e+03) false "None")
        (Utilities|FlowControl|Delay 1.0)
        (CallFunction|ResetTeleportCooldown)))))

(event Input|AxisEvents|InputAxisRight
  (params (AxisValue :type Float%20%28single-precision%29))
  (Pawn|Input|AddMovementInput "0,1.000000, 0" AxisValue false))

(event Input|AxisEvents|InputAxisUp
  (params (AxisValue :type Float%20%28single-precision%29))
  (Pawn|Input|AddMovementInput "1.000000,0.000000, 0" AxisValue false))

(fn ConstructionScript)