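; BP_ChargeShockwave is a shockwave actor, going by its name, that hits players and dice overlapping its Sphere component.
; The overlap event passes each actor to HitPlayers and HitDice, whose bodies are not in this file.
; A custom event tints Sphere1 by applying a dynamic Bubble material with the supplied colour at half strength, then prints a leftover debug "Hello".
; BeginPlay and construction only call the parent.
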(event OnComponentBeginOverlap(Sphere)
  (params (OverlappedComponent :type Primitive%20Component%20Object%20Reference) (OtherActor :type Actor%20Object%20Reference) (OtherComp :type Primitive%20Component%20Object%20Reference) (OtherBodyIndex :type Integer) (bFromSweep :type Boolean) (SweepResult :type Hit%20Result%20Structure%20%28by%20ref%29))
  (CallFunction|HitPlayers OtherActor)
  (CallFunction|HitDice OtherActor))

(event Custom|CustomEvent
  (params (Colour :type Linear%20Color%20Structure))
  (bind _returnvalue (Rendering|Material|CreateDynamicMaterialInstance "/Game/Particles/Materials/Bubble.Bubble" :!class /Script/Engine.KismetMaterialLibrary))
  (Rendering|Material|SetVectorParameterValue _returnvalue "CustomColour" (* Colour 0.5) :!class /Script/Engine.MaterialInstanceDynamic)
  (Rendering|Material|SetMaterial (Variables|Default|GetSphere1) 0 _returnvalue)
  (Development|PrintString "Hello"))

(event EventBeginPlay
  (|CallParentFunction))

(event Collision|EventActorBeginOverlap
  (params (OtherActor :type Actor%20Object%20Reference))
  (|CallParentFunction OtherActor) ; This node is disabled and will not be called.\nDrag off pins to build functionality.
)

(event EventTick
  (params (DeltaSeconds :type Float%20%28single-precision%29))
  (|CallParentFunction DeltaSeconds) ; This node is disabled and will not be called.\nDrag off pins to build functionality.
)

(fn ConstructionScript
  (|CallParentFunction))