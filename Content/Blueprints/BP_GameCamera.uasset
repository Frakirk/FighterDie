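; Game camera actor that keeps a group of tracked objects framed by moving itself each tick.
; It computes the X/Y bounding extents of TrackedObjects, ignoring any that have fallen below a Z cutoff.
; The larger span, with Y scaled for 16:9 aspect, sets how far back along X and how high it sits from the midpoint.
; Movement is smoothed by lerping toward that target using delta seconds.
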(event EventBeginPlay)

(event Collision|EventActorBeginOverlap
  (params (OtherActor :type Actor%20Object%20Reference)))

(event EventTick
  (params (DeltaSeconds :type Float%20%28single-precision%29))
  (Utilities|FlowControl|Sequence
    (:then_0
      (Variables|Default|SetXPosMax -99999.0)
      (Variables|Default|SetXPosMin 99999.0)
      (Variables|Default|SetYPosMax -99999.0)
      (Variables|Default|SetYPosMin 99999.0))
    (:then_1
      (for _array_element (Variables|Default|GetTrackedObjects)
        (if (>= (.Z (Math|Vector|BreakVector (Transformation|GetActorLocation _array_element))) -5e+02)
          (Utilities|FlowControl|Sequence
            (:then_0
              (Variables|Default|SetXPosMax (Math|Float|Max(Float) (Variables|Default|GetXPosMax) (.X (Math|Vector|BreakVector (Transformation|GetActorLocation _array_element)))))
              (Variables|Default|SetXPosMin (Math|Float|Min(Float) (Variables|Default|GetXPosMin) (.X (Math|Vector|BreakVector (Transformation|GetActorLocation _array_element))))))
            (:then_1
              (Variables|Default|SetYPosMax (Math|Float|Max(Float) (Variables|Default|GetYPosMax) (.Y (Math|Vector|BreakVector (Transformation|GetActorLocation _array_element)))))
              (Variables|Default|SetYPosMin (Math|Float|Min(Float) (Variables|Default|GetYPosMin) (.Y (Math|Vector|BreakVector (Transformation|GetActorLocation _array_element))))))))))
    (:then_2
      (Variables|Default|SetXPosMid (* (+ (Variables|Default|GetXPosMin) (Variables|Default|GetXPosMax)) 0.5))
      (Variables|Default|SetYPosMid (* (+ (Variables|Default|GetYPosMin) (Variables|Default|GetYPosMax)) 0.5))
      (Transformation|SetActorLocation (Math|Vector|Lerp(Vector) (Transformation|GetActorLocation) (Math|Vector|MakeVector (- (Variables|Default|GetXPosMid) (* (Math|Float|Max(Float) (Math|Float|Absolute(Float) (- (Variables|Default|GetXPosMax) (Variables|Default|GetXPosMin))) (* (Math|Float|Absolute(Float) (- (Variables|Default|GetYPosMax) (Variables|Default|GetYPosMin))) 0.5625)) 1.625)) (Variables|Default|GetYPosMid) (* (* (Math|Float|Max(Float) (Math|Float|Absolute(Float) (- (Variables|Default|GetXPosMax) (Variables|Default|GetXPosMin))) (* (Math|Float|Absolute(Float) (- (Variables|Default|GetYPosMax) (Variables|Default|GetYPosMin))) 0.5625)) 1.625) 1.6)) (Utilities|Time|GetWorldDeltaSeconds)) false false))))

(fn ConstructionScript)