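; Player controller that routes input either to the CharacterSelectMain widget, when one is on screen, or to the possessed PlayerCharacter.
; On BeginPlay it respawns the pawn in level Test3, otherwise adopts the existing one, colouring it by GameID from BP_GameInstance.
; Number keys hot-swap between Bard, Paladin, Rogue and Wizard through SpawnNewCharacter, and other bindings load levels or quit.
; The GameInstance class lookup is disconnected.
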(event Custom|SpawnNewCharacter
  (bind _returnvalue (Pawn|GetControlledPawn))
  (Variables|Default|SetActorTransform (Transformation|GetActorTransform _returnvalue))
  (Actor|DestroyActor _returnvalue)
  (bind _returnvalue_2 (Game|SpawnActorfromClass (Variables|Default|GetClass) (Variables|Default|GetActorTransform) "Undefined" 0 0))
  (Pawn|Possess _returnvalue_2)
  (bind _outactors (Actor|GetAllActorsOfClass "/Script/Engine.CameraActor"))
  (Game|Player|SetViewTargetwithBlend (Utilities|Array|Get(acopy) _outactors) 0.0 "VTBlend_Linear" 0.0 false)
  (bind _asplayer_character (Utilities|Casting|CastToPlayerCharacter (Pawn|GetControlledPawn)))
  (bind _output_get (Variables|Default|SetPlayerPawn _asplayer_character))
  (Variables|/Game/Blueprints/PlayerCharacter.PlayerCharacter_C|SetControllerRef _output_get self)
  (bind _asbp_game_instance (Utilities|Casting|CastToBP_GameInstance (Game|GetGameInstance)))
  (Default|SetColour _output_get (.Value (Utilities|Map|Find (Variables|/Game/Blueprints/BP_GameInstance.BP_GameInstance_C|GetPlayerColours _asbp_game_instance) (Variables|Default|GetGameID)))))

(event EventBeginPlay
  (bind _asbp_game_instance (Utilities|Casting|CastToBP_GameInstance (Game|GetGameInstance))
    (:then
      (bind _returnvalue (Game|GetCurrentLevelName true))
      (if (Utilities|Enum|Equal(Enum) _returnvalue "Test3")
        (CallFunction|SpawnNewCharacter)
        (else
          (bind _asplayer_character (Utilities|Casting|CastToPlayerCharacter (Pawn|GetControlledPawn)))
          (bind _output_get (Variables|Default|SetPlayerPawn _asplayer_character))
          (Variables|/Game/Blueprints/PlayerCharacter.PlayerCharacter_C|SetControllerRef _output_get self)
          (bind _asbp_game_instance_2 (Utilities|Casting|CastToBP_GameInstance (Game|GetGameInstance)))
          (Default|SetColour _output_get (.Value (Utilities|Map|Find (Variables|/Game/Blueprints/BP_GameInstance.BP_GameInstance_C|GetPlayerColours _asbp_game_instance_2) (Variables|Default|GetGameID)))))))
    (:CastFailed
      (Development|PrintString "FAILED TO FIND GAME INSTANCE"))))

(event Input|ActionEvents|InputActionAbilityX
  (params (Key :type Key%20Structure))
  (bind _playerpawn (Variables|Default|GetPlayerPawn))
  (:Pressed
    (Default|InputXPress _playerpawn))
  (:Released
    (Utilities|CheckifCharacterSelect
      (:False
        (Default|InputXRelease _playerpawn)))))

(event Input|ActionEvents|InputActionStart
  (params (Key :type Key%20Structure))
  (:Pressed
    (bind _characterselectwidget (Utilities|CheckifCharacterSelect)
      (:True
        (Default|InputStart _characterselectwidget)))))

(event Input|ActionEvents|InputActionAbilityB
  (params (Key :type Key%20Structure))
  (:Pressed
    (bind _characterselectwidget (Utilities|CheckifCharacterSelect)
      (:True
        (Default|InputB _characterselectwidget self)))))

(event Input|ActionEvents|InputActionQuit
  (params (Key :type Key%20Structure))
  (:Pressed
    (Game|QuitGame 0 "Quit")))

(event Input|ActionEvents|InputActionAbilityA
  (params (Key :type Key%20Structure))
  (:Pressed
    (bind _characterselectwidget (Utilities|CheckifCharacterSelect)
      (:True
        (Default|InputA _characterselectwidget self))
      (:False
        (Default|InputAPress (Variables|Default|GetPlayerPawn)))))
  (:Released
    (Utilities|CheckifCharacterSelect
      (:False
        (Default|InputARelease (Variables|Default|GetPlayerPawn))))))

(event Input|AxisEvents|InputAxisRight
  (params (AxisValue :type Float%20%28single-precision%29))
  (bind _playerpawn (Variables|Default|GetPlayerPawn))
  (bind _characterselectwidget (Utilities|CheckifCharacterSelect)
    (:True
      (Math|Float|CompareFloat (Math|Float|Absolute(Float) AxisValue) 0.5
        (:>
          (Utilities|FlowControl|DoOnce false :!label _label
            (:Completed
              (Math|Float|CompareFloat (Input|AxisValues|GetRight) 0.0
                (:>
                  (Default|NextCharacter _characterselectwidget self))
                (:<
                  (Default|PreviousCharacter _characterselectwidget self))))))
        (:<
          (goto _label Reset))))
    (:False
      (Utilities|IsValid _playerpawn
        (:Is%20Valid
          (Default|MoveLeftRight _playerpawn AxisValue))))))

(event Input|AxisEvents|InputAxisUp
  (params (AxisValue :type Float%20%28single-precision%29))
  (bind _playerpawn (Variables|Default|GetPlayerPawn))
  (Utilities|CheckifCharacterSelect
    (:False
      (Utilities|IsValid _playerpawn
        (:Is%20Valid
          (Default|MoveUpDown _playerpawn AxisValue))))))

(event Input|KeyboardEvents|R
  (params (Key :type Key%20Structure))
  (:Pressed
    (Game|OpenLevel(byName) "Menu")))

(event Input|KeyboardEvents|X
  (params (Key :type Key%20Structure))
  (:Pressed
    (Game|OpenLevel(byName) "TestMap")))

(event Input|GamepadEvents|GamepadSpecialLeft
  (params (Key :type Key%20Structure))
  (:Pressed
    (Game|OpenLevel(byName) "Menu")))

(event Input|KeyboardEvents|2
  (params (Key :type Key%20Structure))
  (:Pressed
    (Variables|Default|SetClass "/Game/Blueprints/PlayerClasses/BP_PlayerPaladin.BP_PlayerPaladin_C")
    (CallFunction|SpawnNewCharacter)))

(event Input|KeyboardEvents|3
  (params (Key :type Key%20Structure))
  (:Pressed
    (Variables|Default|SetClass "/Game/Blueprints/PlayerClasses/BP_PlayerRogue.BP_PlayerRogue_C")
    (CallFunction|SpawnNewCharacter)))

(event Input|KeyboardEvents|4
  (params (Key :type Key%20Structure))
  (:Pressed
    (Variables|Default|SetClass "/Game/Blueprints/PlayerClasses/BP_PlayerWizard.BP_PlayerWizard_C")
    (CallFunction|SpawnNewCharacter)))

(event Input|KeyboardEvents|1
  (params (Key :type Key%20Structure))
  (:Pressed
    (Variables|Default|SetClass "/Game/Blueprints/PlayerClasses/BP_PlayerBard.BP_PlayerBard_C")
    (CallFunction|SpawnNewCharacter)))

(fn ConstructionScript)

(fn GetInputAxes
  (return (Input|AxisValues|GetUp) (Input|AxisValues|GetRight)))

(fn IsActive
  (Math|Integer|CompareInt (Variables|Default|GetGameID) -1
    (:>
      (return true))
    (:==
      _)
    (:<
      _))
  (return false))