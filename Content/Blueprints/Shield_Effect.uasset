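; Shield_Effect is a short-lived effect actor that spins and shrinks until it disappears.
; Each Tick sets the yaw from a Rotate counter, which grows by a fixed step and wraps to zero after a full turn.
; Tick also applies a uniform scale that drops by a fixed step and destroys the actor once it reaches zero or below.
; Both steps ignore delta time, so speed and lifetime depend on frame rate.
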(event EventBeginPlay)

(event Collision|EventActorBeginOverlap
  (params (OtherActor :type Actor%20Object%20Reference)))

(event EventTick
  (params (DeltaSeconds :type Float%20%28single-precision%29))
  (Transformation|SetActorRotation (Math|Rotator|MakeRotator 0.0 0.0 (Variables|Default|GetRotate)))
  (bind _output_get (Variables|Default|SetRotate (+ (Variables|Default|GetRotate) 3.0)))
  (Math|Float|CompareFloat _output_get 3.6e+02
    (:>
      (Variables|Default|SetRotate 0.0 :!label _label))
    (:==
      (goto _label))
    (:<
      _))
  (Transformation|SetActorScale3D (Math|Vector|MakeVector (Variables|Default|GetScale) (Variables|Default|GetScale) (Variables|Default|GetScale)))
  (bind _output_get_2 (Variables|Default|SetScale (- (Variables|Default|GetScale) 0.01)))
  (Math|Float|CompareFloat _output_get_2 0.0
    (:==
      _)
    (:<
      _))
  (Actor|DestroyActor))

(fn ConstructionScript)