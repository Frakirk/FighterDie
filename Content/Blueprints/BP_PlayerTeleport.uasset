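; BP_PlayerTeleport is a physics-driven actor that teleports its owner to wherever it is after a two-second delay, then destroys itself.
; Each tick it damps the Sphere's linear velocity by lerping toward zero with a fixed, frame-rate-dependent alpha.
; Teleport places the owner at a fixed offset below the actor's location, without sweeping.
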(event Custom|Teleport
  (Transformation|SetActorLocation (Components|GetOwner) (+ (Transformation|GetActorLocation) "0, 0,-150.000000") false false)
  (Actor|DestroyActor))

(event EventBeginPlay
  (Utilities|FlowControl|Delay 2.0)
  (CallFunction|Teleport))

(event EventTick
  (params (DeltaSeconds :type Float%20%28single-precision%29))
  (bind _sphere (Variables|Default|GetSphere))
  (bind _returnvalue (Physics|GetPhysicsLinearVelocity _sphere "None"))
  (Physics|SetPhysicsLinearVelocity _sphere (Math|Vector|Lerp(Vector) _returnvalue "0.000000, 0, 0" 0.075) false "None"))

(fn ConstructionScript)