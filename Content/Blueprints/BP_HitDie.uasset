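; BP_HitDie is a physics die standing in for its instigating player, whose input it disables and colour it copies while the camera tracks it.
; BeginPlay places it outward along the player's direction and lobs it toward the origin with random spin.
; Player hits bounce it, launch that character and play a debounced bump sound.
; Once nearly still, it teleports the player there, resets their time dilation and self-destructs, restoring input and camera tracking.
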(event OnComponentHit(Cube)
  (params (HitComponent :type Primitive%20Component%20Object%20Reference) (OtherActor :type Actor%20Object%20Reference) (OtherComp :type Primitive%20Component%20Object%20Reference) (NormalImpulse :type Vector :default "0, 0, 0") (Hit :type Hit%20Result%20Structure%20%28by%20ref%29))
  (if (not (Variables|Default|GetHasBumpPlayed))
    (bind _asplayer_character (Utilities|Casting|CastToPlayerCharacter OtherActor))
    (CallFunction|Bounce _asplayer_character 1.0)
    (Character|LaunchCharacter _asplayer_character (Math|Vector|MakeVector (.X (Math|Vector|BreakVector (* (Math|Vector|GetUnitDirection(Vector) (Transformation|GetWorldLocation (Variables|Default|GetCube)) (Transformation|GetActorLocation _asplayer_character)) 2.5e+02))) (.Y (Math|Vector|BreakVector (* (Math|Vector|GetUnitDirection(Vector) (Transformation|GetWorldLocation (Variables|Default|GetCube)) (Transformation|GetActorLocation _asplayer_character)) 2.5e+02))) 5e+01) true true)
    (CallFunction|DiceBumpSound)))

(event Custom|Bounce
  (params (OtherActor :type Actor%20Object%20Reference) (ForceScale :type Float%20%28single-precision%29))
  (bind _returnvalue (Transformation|GetActorLocation OtherActor))
  (bind _cube (Variables|Default|GetCube))
  (bind _returnvalue_2 (Transformation|GetWorldLocation _cube))
  (bind (_x _y) (Math|Vector|BreakVector _returnvalue))
  (bind (_x_2 _y_2) (Math|Vector|BreakVector _returnvalue_2))
  (Physics|SetPhysicsLinearVelocity (Variables|Default|GetCube) (* (Math|Vector|GetUnitDirection(Vector) (Math|Vector|MakeVector _x _y 0.0) (Math|Vector|MakeVector _x_2 _y_2 2.5e+02)) (* ForceScale 1e+03)) true "None")
  (Class|PrimitiveComponent|SetPhysicsAngularVelocityinDegrees (Variables|Default|GetCube) (* (Math|Random|RandomUnitVector) 2.5e+02) true "None"))

(event Custom|DiceBumpSound
  (bind _returnvalue (Transformation|GetActorLocation))
  (bind _returnvalue_2 (Math|Random|RandomFloatinRange 0.8 0.9))
  (bind _volumelevel (Variables|Default|GetVolumeLevel))
  (switch int (Math|Random|RandomIntegerinRange 0 3)
    (:0
      (Audio|SpawnSoundatLocation "/Game/Sound/Effects/PaladinStep1.PaladinStep1" _returnvalue "0, 0, 0" _volumelevel _returnvalue_2 _returnvalue_2))
    (:1
      (Audio|SpawnSoundatLocation "/Game/Sound/Effects/PaladinStep1.PaladinStep1" _returnvalue "0, 0, 0" _volumelevel _returnvalue_2))
    (:2
      (Audio|SpawnSoundatLocation "/Game/Sound/Effects/PaladinStep1.PaladinStep1" _returnvalue "0, 0, 0" _volumelevel _returnvalue_2))
    (:3
      (Audio|SpawnSoundatLocation "/Game/Sound/Effects/PaladinStep1.PaladinStep1" _returnvalue "0, 0, 0" _volumelevel _returnvalue_2)))
  (Variables|Default|SetHasBumpPlayed true)
  (Utilities|FlowControl|Delay 0.1)
  (Variables|Default|SetHasBumpPlayed false))

(event Collision|EventActorBeginOverlap
  (params (OtherActor :type Actor%20Object%20Reference)))

(event EventTick
  (params (DeltaSeconds :type Float%20%28single-precision%29))
  (bind _instigator (Variables|Default|GetInstigator))
  (Math|Float|CompareFloat (.z (Transformation|GetActorLocation)) -5e+03
    (:>
      _)
    (:==
      _)
    (:<
      _))
  (bind _returnvalue (Physics|GetPhysicsLinearVelocity (Variables|Default|GetCube) "None"))
  (Math|Float|CompareFloat (Math|Vector|VectorLength _returnvalue) 0.01
    (:>
      (goto _label Reset))
    (:<
      (Utilities|FlowControl|DoOnce true :!label _label
        (:Completed
          (Transformation|SetActorLocation _instigator (Transformation|GetActorLocation) false false)
          (Variables|/Script/Engine.Actor|SetCustomTimeDilation _instigator 1.0)
          (Actor|DestroyActor))))))

(event EventDestroyed
  (bind _outactors (Actor|GetAllActorsOfClass "/Game/Blueprints/BP_GameCamera.BP_GameCamera_C"))
  (Utilities|Array|RemoveItem (Variables|/Game/Blueprints/BP_GameCamera.BP_GameCamera_C|GetTrackedObjects (Utilities|Array|Get(acopy) _outactors)) self)
  (bind _asplayer_controller (Utilities|Casting|CastToPlayerController (Pawn|GetController (Variables|Default|GetInstigator))))
  (Input|EnableInput _asplayer_controller _asplayer_controller))

(event EventBeginPlay
  (bind _returnvalue (Transformation|GetActorLocation))
  (bind _instigator (Variables|Default|GetInstigator))
  (bind _returnvalue_2 (Transformation|GetActorLocation _instigator))
  (bind _returnvalue_3 (* _returnvalue -1.0))
  (bind (_x _y) (Math|Vector|BreakVector _returnvalue_3))
  (bind _returnvalue_4 (* _returnvalue_2 "1.000000,1.000000, 0"))
  (bind _returnvalue_5 (Math|Vector|Normalize _returnvalue_4))
  (bind _returnvalue_6 (* _returnvalue_5 2e+03))
  (bind (_x_2 _y_2) (Math|Vector|BreakVector _returnvalue_6))
  (Transformation|SetActorLocation (Math|Vector|MakeVector _x_2 _y_2 5e+02) false false)
  (Physics|SetPhysicsLinearVelocity (Variables|Default|GetCube) (+ (* (Math|Vector|Normalize (Math|Vector|MakeVector _x _y 0.0)) (Math|Vector|VectorLength _returnvalue)) "0, 0,1500.000000") false "None")
  (Class|PrimitiveComponent|SetPhysicsAngularVelocityinDegrees (Variables|Default|GetCube) (* (Math|Random|RandomUnitVector) 1e+03) false "None")
  (bind _asplayer_character (Utilities|Casting|CastToPlayerCharacter (Variables|Default|GetInstigator)))
  (CallFunction|SetColour (Variables|/Game/Blueprints/PlayerCharacter.PlayerCharacter_C|GetColour _asplayer_character))
  (bind _asplayer_controller (Utilities|Casting|CastToPlayerController (Pawn|GetController _asplayer_character)))
  (Input|DisableInput _asplayer_controller _asplayer_controller)
  (bind _outactors (Actor|GetAllActorsOfClass "/Game/Blueprints/BP_GameCamera.BP_GameCamera_C"))
  (Utilities|Array|AddUnique (Variables|/Game/Blueprints/BP_GameCamera.BP_GameCamera_C|GetTrackedObjects (Utilities|Array|Get(acopy) _outactors)) self))

(fn ConstructionScript
  (|CallParentFunction))